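; Animation notify state that deals sword attack damage from a BP_BaseCharacter during the notify window.
; Each tick it sphere-traces on the Camera channel between the mesh's sword start and end sockets.
; A hit BP_BaseCharacter receives the attacker's last attack damage and joins DamageCharacters.
; That list is cleared on notify begin, limiting each target to one hit per window.
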(fn ReceivedNotifyTick
  (params (MeshComp :type Skeletal%20Mesh%20Component%20Object%20Reference) (Animation :type Anim%20Sequence%20Base%20Object%20Reference) (FrameDeltaTime :type Float%20%28single-precision%29) (EventReference :type Anim%20Notify%20Event%20Reference%20Structure%20%28by%20ref%29))
  (bind _asbp_base_character (Utilities|Casting|CastToBP_BaseCharacter (Components|GetOwner MeshComp))
    (:then
      (bind _outhit (Collision|SphereTraceByChannel MeshComp (Transformation|GetSocketLocation MeshComp "SwordAttackSocketStart") (Transformation|GetSocketLocation MeshComp "SwordAttackSocketEnd") 5.0 "TraceTypeQuery2" false 0 "None" true "(R=1.000000,G=0.000000,B=0.000000,A=1.000000)" "(R=0.000000,G=1.000000,B=0.000000,A=1.000000)" 1.0))
      (bind _asbp_base_character_2 (Utilities|Casting|CastToBP_BaseCharacter (.HitActor (Collision|BreakHitResult _outhit)))
        (:then
          (if (not (Utilities|Array|ContainsItem (Variables|Default|GetDamageCharacters) _asbp_base_character_2))
            (Utilities|Array|Add (Variables|Default|GetDamageCharacters) _asbp_base_character_2)
            (Game|Damage|ApplyDamage _asbp_base_character_2 (Variables|/Game/Game/Blueprints/Characters/BP_BaseCharacter.BP_BaseCharacter_C|GetBLastAttackDamage _asbp_base_character) 0 0)
            (return true)))
        (:CastFailed
          (return false))))
    (:CastFailed
      (return false))))

(fn ReceivedNotifyBegin
  (params (MeshComp :type Skeletal%20Mesh%20Component%20Object%20Reference) (Animation :type Anim%20Sequence%20Base%20Object%20Reference) (TotalDuration :type Float%20%28single-precision%29) (EventReference :type Anim%20Notify%20Event%20Reference%20Structure%20%28by%20ref%29))
  (Utilities|Array|Clear (Variables|Default|GetDamageCharacters))
  (return false))