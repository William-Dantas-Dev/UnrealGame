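; Base character Blueprint for sword combat, handling attacking, health and death.
; On BeginPlay it spawns a BP_Sword and attaches it to the mesh's SwordSocket.
; Attacks are gated on not attacking or falling, then store a random damage value and play a montage; jumping is also blocked while attacking.
; Incoming damage reduces clamped health; at zero, a valid sword is destroyed and the mesh ragdolls.
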(event Custom|Attack_Event
  (if (CallFunction|CanAttack?)
    (Variables|Default|SetbIsAttacking true)
    (Variables|Default|SetBLastAttackDamage (Math|Conversions|ToFloat(Integer) (Math|Random|RandomIntegerinRange 25 50)))
    (Animation|PlayAnimMontage "/Game/Game/Animations/Attack/AttackAnim/AM_Attack1.AM_Attack1" 1.0 "Default")))

(event EventBeginPlay
  (CallFunction|GetSword))

(event Game|Damage|EventAnyDamage
  (params (Damage :type Float%20%28single-precision%29) (DamageType :type Damage%20Type%20Object%20Reference) (InstigatedBy :type Controller%20Object%20Reference) (DamageCauser :type Actor%20Object%20Reference))
  (bind _mesh (Variables|Character|GetMesh))
  (bind _output_get (Variables|Default|SetHealth (Math|Float|Clamp(Float) (- (Variables|Default|GetHealth) Damage) 0.0 1e+02)))
  (if (> _output_get 0.0)
    (Development|PrintString (Utilities|String|ToString(Float) (Variables|Default|GetHealth)))
    (else
      (bind _sword (Variables|Default|GetSword)
        (:then
          (Actor|DestroyActor _sword)
          (Collision|SetCollisionEnabled _mesh "QueryAndPhysics")
          (Physics|SetSimulatePhysics _mesh true))
        (:else)))))

(fn ConstructionScript)

(fn GetSword
  ;[1 1 1] Get And Attach Sword
  (bind _returnvalue (Game|SpawnActorfromClass "/Game/Game/Blueprints/Weapons/BP_Sword.BP_Sword_C" (Math|Transform|MakeTransform "0, 0, 0") "Undefined" "MultiplyWithRoot" 0 0))
  (bind _output_get (Variables|Default|SetSword _returnvalue))
  (Transformation|AttachComponentToComponent _output_get (Variables|Character|GetMesh) "SwordSocket" "KeepRelative" "KeepRelative" "KeepRelative" true))

(fn SetIsAttack
  (params (IsAttacking :type Boolean))
  (Variables|Default|SetbIsAttacking IsAttacking))

(fn CanAttack?
  (return (and (not (Variables|Default|GetbIsAttacking)) (not (AI|Components|NavMovement|IsFalling (Variables|Character|GetCharacterMovement))))))

(fn CanJump?
  (return (not (Variables|Default|GetbIsAttacking))))